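; Tree actor that falls when hit by an actor tagged "Axe" and completes the "Chop" quest.
; The tree mesh's hit event, gated by a DoOnce, stores the starting relative transforms of tree and stump, then plays the TreeFall timeline.
; Separate timeline tracks lerp each mesh toward its target transform.
; When the timeline finishes, the quest manager completes the whole quest.
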(event OnComponentHit(Tree_Mesh)
  (params (HitComponent :type Primitive%20Component%20Object%20Reference) (OtherActor :type Actor%20Object%20Reference) (OtherComp :type Primitive%20Component%20Object%20Reference) (NormalImpulse :type Vector :default "0, 0, 0") (Hit :type Hit%20Result%20Structure%20%28by%20ref%29))
  (if (Actor|ActorHasTag OtherActor "Axe")
    (Utilities|FlowControl|DoOnce false
      (:Completed
        (Variables|Default|SetStartRotation (Transformation|GetRelativeTransform (Variables|Default|GetTree_Mesh)))
        (Variables|Default|SetStartStump (Transformation|GetRelativeTransform (Variables|Default|GetSM_Treestump_Var01)))
        (bind (_direction _tree _stump) (Timeline|Tree%20Fall Play)
          (:Update
            (Utilities|FlowControl|Sequence
              (:then_0
                (Transformation|SetRelativeTransform (Variables|Default|GetTree_Mesh) (Math|Transform|Lerp(Transform) (Variables|Default|GetStartRotation) (Variables|Default|GetTargetRotation) _tree) false false))
              (:then_1
                (Transformation|SetRelativeTransform (Variables|Default|GetSM_Treestump_Var01) (Math|Transform|Lerp(Transform) (Variables|Default|GetStartStump) (Variables|Default|GetTargetStump) _stump) false false))))
          (:Finished
            (Class|QuestManager|CompleteQuest (CallFunction|GetQuestManager) "Chop" true)))))))

(event EventBeginPlay
  (|CallParentFunction) ; This node is disabled and will not be called.\nDrag off pins to build functionality.
)

(event Collision|EventActorBeginOverlap
  (params (OtherActor :type Actor%20Object%20Reference))
  (|CallParentFunction OtherActor) ; This node is disabled and will not be called.\nDrag off pins to build functionality.
)

(event EventTick
  (params (DeltaSeconds :type Float%20%28single-precision%29))
  (|CallParentFunction DeltaSeconds) ; This node is disabled and will not be called.\nDrag off pins to build functionality.
)

(fn ConstructionScript
  (|CallParentFunction))