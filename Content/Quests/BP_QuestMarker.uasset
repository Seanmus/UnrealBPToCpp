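; Quest marker Blueprint that shows a Niagara effect while a named quest is active and at a specific progress value.
; On BeginPlay it binds to the quest manager's completed-quest event and sets its initial visibility.
; Each event re-runs RefreshVisibility, which looks up the quest by QuestName and compares its progress to ShowAtProgress, avoiding Tick polling.
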(event Custom|Quest%20Updated
  (params (Index :type Integer))
  (CallFunction|RefreshVisibility))

(event EventBeginPlay
  (EventDispatchers|BindEventtoCompletedQuest (CallFunction|GetQuestManager) (delegate Custom|Quest%20Updated))
  (CallFunction|RefreshVisibility))

(event Collision|EventActorBeginOverlap
  (params (OtherActor :type Actor%20Object%20Reference)))

(event EventTick
  (params (DeltaSeconds :type Float%20%28single-precision%29)))

(fn ConstructionScript)

(fn RefreshVisibility
  (bind _questmanager (CallFunction|GetQuestManager))
  (bind _questname (Variables|Default|GetQuestName))
  (bind _quest (Default|GetQuest _questmanager _questname))
  (Rendering|SetVisibility (Variables|Default|GetNiagaraSystem) (and (Default|IsActiveQuest _questmanager (.questid _quest)) (== (.progress _quest) (Variables|Default|GetShowAtProgress))) false))